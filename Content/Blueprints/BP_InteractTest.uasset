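; BP_InteractTest is an interactable test actor that destroys itself when interacted with.
; Its Collision overlap events show the WBPInteractableUI prompt and set the actor as InteractableActor on the overlapping BP_FirstPersonCharacter.
; Ending the overlap hides the prompt and sets that reference to None, without checking whether another interactable has replaced it.
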(event `/Game/Blueprints/BPI_InteractableActor.OnInteract`
  (`self.K2_DestroyActor`))

(event `self.Collision.OnComponentBeginOverlap`
  (params (OverlappedComponent :type "PrimitiveComponent Object Reference") (OtherActor :type "Actor Object Reference") (OtherComp :type "PrimitiveComponent Object Reference") (OtherBodyIndex :type Integer) (bFromSweep :type Boolean) (SweepResult :type "HitResult Structure (by ref)"))
  (bind _asbp_first_person_character (cast `/Game/FirstPerson/Blueprints/BP_FirstPersonCharacter` OtherActor))
  (`SceneComponent.SetVisibility` (`self.WBP_InteractableUI`) true false)
  (set `/Game/FirstPerson/Blueprints/BP_FirstPersonCharacter.InteractableActor` self _asbp_first_person_character))

(event `self.Collision.OnComponentEndOverlap`
  (params (OverlappedComponent :type "PrimitiveComponent Object Reference") (OtherActor :type "Actor Object Reference") (OtherComp :type "PrimitiveComponent Object Reference") (OtherBodyIndex :type Integer))
  (bind _asbp_first_person_character (cast `/Game/FirstPerson/Blueprints/BP_FirstPersonCharacter` OtherActor))
  (`SceneComponent.SetVisibility` (`self.WBP_InteractableUI`) false false)
  (set `/Game/FirstPerson/Blueprints/BP_FirstPersonCharacter.InteractableActor` null _asbp_first_person_character))

(fn `UserConstructionScript`)